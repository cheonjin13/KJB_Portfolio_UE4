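; Player skill tree component that manages skill points, spell learning and stage changes, and toggles the tree widget with the matching input mode and cursor.
; Upgrades check points, character level and prerequisite spells, with first-stage unlocks recording the class on BP_PlayerBase and activating its tree connections.
; Downgrades step a stage back and refund a point.
; Changes refresh the widget's entries and point display, and a helper finds a skill's hotkey slot.
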(event `self.ReceiveBeginPlay`
  (bind _asbp_player_base (cast `/Game/MyContents/Character/BP_PlayerBase` (`self.GetOwner`)))
  (set `self.PlayerCharacter` _asbp_player_base))

(event `SetupTree`
  (bind _output_get (set `self.TreeWidget` (`/Game/MyContents/UI/UI_PlayerBagic.SkillTree` (`/Game/MyContents/Character/BP_PlayerBase.MainWidget` (`self.PlayerCharacter`)))))
  (`/Game/MyContents/SkillSystem/UI/W_MainTree.Initialize` _output_get self)
  (set `self.TreeSetup` true))

(event `HandleShowCommand`
  (bind _treewidget (`self.TreeWidget`))
  (bind _playerconref (`/Game/MyContents/Character/BP_PlayerBase.PlayerConRef` (`self.PlayerCharacter`)))
  (if (`self.TreeSetup`)
    (if (`self.TreeShown`)
      (`Widget.SetVisibility` (`self.TreeWidget`) "Hidden")
      (`WidgetBlueprintLibrary.SetInputMode_GameOnly` _playerconref)
      (set `PlayerController.bShowMouseCursor` false _playerconref)
      (set `self.TreeShown` false)
      (else
        (`Widget.SetVisibility` _treewidget "SelfHitTestInvisible")
        (`WidgetBlueprintLibrary.SetInputMode_GameAndUIEx` _playerconref _treewidget "DoNotLock" false)
        (set `PlayerController.bShowMouseCursor` true _playerconref)
        (set `self.TreeShown` true)))))

(event `DowngradeSpell`
  (params (SkillActor :type "/Game/MyContents/SkillSystem/SkillActors/Master_Skill Object Reference") (EntryWidget :type "/Game/MyContents/SkillSystem/UI/W_SkillTreeEntry Object Reference"))
  (bind _upgradedspell (`self.UpgradedSpell`))
  (bind _entrywidget (`self.EntryWidget`))
  (set `self.UpgradedSpell` SkillActor)
  (set `self.EntryWidget` EntryWidget)
  (set `/Game/MyContents/SkillSystem/SkillActors/Master_Skill.CurrentStageIndex` (- (`/Game/MyContents/SkillSystem/SkillActors/Master_Skill.CurrentStageIndex` _upgradedspell) 1) _upgradedspell)
  (`/Game/MyContents/SkillSystem/UI/W_SkillTreeEntry.UpdateStageText` _entrywidget)
  (`/Game/MyContents/SkillSystem/UI/W_SkillTreeEntry.UpdateIcon` _entrywidget)
  (`self.AddSkillPoints` 1)
  (`self.UpdateAllEntries`))

(event `UpgradeSpell`
  (params (SkillActor :type "/Game/MyContents/SkillSystem/SkillActors/Master_Skill Object Reference") (EntryWidget :type "/Game/MyContents/SkillSystem/UI/W_SkillTreeEntry Object Reference"))
  (bind _upgradedspell (`self.UpgradedSpell`))
  (bind _entrywidget (`self.EntryWidget`))
  (bind _returnvalue (`GameplayStatics.GetObjectClass` (`self.UpgradedSpell`)))
  (bind _output_get (set `self.UpgradedSpell` SkillActor))
  (set `self.EntryWidget` EntryWidget)
  (bind _out (`self.CanUpgradeSpell` _output_get))
  (if _out
    (set `self.SkillPoints` (- (`self.SkillPoints`) 1))
    (bind _output_get_2 (set `/Game/MyContents/SkillSystem/SkillActors/Master_Skill.CurrentStageIndex` (+ (`/Game/MyContents/SkillSystem/SkillActors/Master_Skill.CurrentStageIndex` _upgradedspell) 1) _upgradedspell))
    (if (== _output_get_2 0)
      (`BlueprintSetLibrary.Set_Add` (`/Game/MyContents/Character/BP_PlayerBase.LearntSpellClasses` (`self.PlayerCharacter`)) _returnvalue)
      (`/Game/MyContents/SkillSystem/UI/W_SkillTreeEntry.OnSpellLearned` (`self.EntryWidget`))
      (`self.ActivateConnections` _returnvalue))
    (`/Game/MyContents/SkillSystem/UI/W_SkillTreeEntry.UpdateStageText` _entrywidget)
    (`/Game/MyContents/SkillSystem/UI/W_SkillTreeEntry.UpdateIcon` _entrywidget)
    (`/Game/MyContents/SkillSystem/UI/W_MainTree.UpdateSP` (`self.TreeWidget`))
    (`self.UpdateAllEntries`)))

(fn `ActivateConnections`
  (params (ForSpell :type "/Game/MyContents/SkillSystem/SkillActors/Master_Skill Class Reference"))
  (locals (localSpell :type "/Game/MyContents/SkillSystem/SkillActors/Master_Skill Class Reference"))
  (set `local.localSpell` ForSpell)
  (for _array_element (`/Game/MyContents/SkillSystem/UI/W_MainTree.SubTreeWidgets` (`self.TreeWidget`))
    (for _array_element_2 (`/Game/MyContents/SkillSystem/UI/W_SubTree.Connections` _array_element)
      (if (== (`/Game/MyContents/SkillSystem/UI/W_Connection.ForSpell` _array_element_2) (`local.localSpell`))
        (`/Game/MyContents/SkillSystem/UI/W_Connection.Activate` _array_element_2)))))

(fn `AddSkillPoints`
  (params (Amount :type Integer))
  (set `self.SkillPoints` (+ (`self.SkillPoints`) Amount))
  (`self.UpdateAllEntries`)
  (`/Game/MyContents/SkillSystem/UI/W_MainTree.UpdateSP` (`self.TreeWidget`)))

(fn `CanUpgradeSpell`
  (params (Spell :type "/Game/MyContents/SkillSystem/SkillActors/Master_Skill Object Reference"))
  (returns (Out :type Boolean))
  (locals (localBool :type Boolean :default true))
  (bind ((`RequiredLevel_2_E91DBBAE4E3E1034918F578758ACADFD` _requiredlevel) (`RequiredSkills_6_6B90C1234F96398A2C5C0B95260B3D9B` _requiredskills)) (break `/Game/MyContents/SkillSystem/Structures/S_SkillStage` (`/Game/MyContents/SkillSystem/SkillActors/Master_Skill.NextStage` Spell)))
  (if (and (> (`self.SkillPoints`) 0) (>= (`MyCharacterDataComponent.GetCurrentCharacterLevel` (`MyCharacter.CharacterStat` (`self.PlayerCharacter`))) _requiredlevel) (< (`/Game/MyContents/SkillSystem/SkillActors/Master_Skill.CurrentStageIndex` Spell) (`KismetArrayLibrary.Array_LastIndex` (`.Stages_12_2F1FC72048A16AA236AD4796F9D85D34` (break `/Game/MyContents/SkillSystem/Structures/S_SkillInfo` (`/Game/MyContents/SkillSystem/SkillActors/Master_Skill.SkillInfo` Spell))))))
    (for _array_element _requiredskills
      (if (not (`self.PlayerLearntSpell` _array_element))
        (set `local.localBool` false)
        (break)))
    (return (`local.localBool`))
    (else
      (return false))))

(fn `PlayerLearntSpell`
  (params (Spell :type "/Game/MyContents/SkillSystem/SkillActors/Master_Skill Class Reference"))
  (returns (out :type Boolean))
  (return (`BlueprintSetLibrary.Set_Contains` (`/Game/MyContents/Character/BP_PlayerBase.LearntSpellClasses` (`self.PlayerCharacter`)) Spell)))

(fn `SkillOnHotkey`
  (params (Skill :type "/Game/MyContents/SkillSystem/SkillActors/Master_Skill Object Reference"))
  (returns (Out :type Boolean) (Hotkey :type "/Game/MyContents/SkillSystem/UI/W_SkillHotKey Object Reference"))
  (locals (localSkill :type "/Game/MyContents/SkillSystem/SkillActors/Master_Skill Object Reference") (localOut :type Boolean) (localHotkey :type "/Game/MyContents/SkillSystem/UI/W_SkillHotKey Object Reference"))
  (set `local.localSkill` Skill)
  (for _array_element (`/Game/MyContents/UI/UI_PlayerBagic.AllHotkeySlots` (`/Game/MyContents/Character/BP_PlayerBase.MainWidget` (`self.PlayerCharacter`)))
    (bind _assignedspell_ (`/Game/MyContents/SkillSystem/UI/W_SkillHotKey.AssignedSpell ` _array_element))
    (`/Engine/EditorBlueprintResources/StandardMacros.IsValid` _assignedspell_
      (:`Is Valid`
        (if (== _assignedspell_ (`local.localSkill`))
          (set `local.localOut` true)
          (set `local.localHotkey` _array_element)
          (break)))))
  (return (`local.localOut`) (`local.localHotkey`)))

(fn `UpdateAllEntries`
  (for _array_element (`/Game/MyContents/SkillSystem/UI/W_MainTree.SubTreeWidgets` (`self.TreeWidget`))
    (for _array_element_2 (`/Game/MyContents/SkillSystem/UI/W_SubTree.SkillEntries` _array_element)
      (`/Game/MyContents/SkillSystem/UI/W_SkillTreeEntry.UpdateUpgradeBox` _array_element_2))))