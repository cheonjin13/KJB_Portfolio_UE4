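; Magic projectile actor fired by a player skill, damaging the first monster it hits.
; On BeginPlay it sets projectile movement speed from the skill's current stage and applies the missile particle effect.
; When its sphere overlaps a Monster, it spawns the impact effect, deals stage damage credited to the skill's player and controller, then destroys itself.
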(event `self.ReceiveBeginPlay`
  (bind _projectilemovement (`self.ProjectileMovement`))
  (bind ((`MissileSpeed_23_1DEF2B4244C20DD53E17938064D8C830` _missilespeed)) (break `/Game/MyContents/SkillSystem/Structures/S_SkillStage` (`/Game/MyContents/SkillSystem/SkillActors/Master_Skill.GetCurrentStage` (`self.Skill`))))
  (set `ProjectileMovementComponent.InitialSpeed` _missilespeed _projectilemovement)
  (set `ProjectileMovementComponent.MaxSpeed` _missilespeed _projectilemovement)
  (`ParticleSystemComponent.SetTemplate` (`self.ParticleSystem`) (`self.MissileEffect`)))

(event `self.Sphere.OnComponentBeginOverlap`
  (params (OverlappedComponent :type "PrimitiveComponent Object Reference") (OtherActor :type "Actor Object Reference") (OtherComp :type "PrimitiveComponent Object Reference") (OtherBodyIndex :type Integer) (bFromSweep :type Boolean) (SweepResult :type "HitResult Structure (by ref)"))
  (bind _playerref (`/Game/MyContents/SkillSystem/SkillActors/Master_Skill.PlayerRef` (`self.Skill`)))
  (bind _asmonster (cast `Monster` OtherActor))
  (`GameplayStatics.SpawnEmitterAtLocation` (`self.ImpactEffect`) (`self.K2_GetActorLocation`))
  (`Monster.TakeDamage` _asmonster (`.Damage_15_FE7E19D842CF09CBD9F3D183294FBD70` (break `/Game/MyContents/SkillSystem/Structures/S_SkillStage` (`/Game/MyContents/SkillSystem/SkillActors/Master_Skill.GetCurrentStage` (`self.Skill`)))) (make `DamageEvent`) (`Pawn.GetController` _playerref) _playerref)
  (`self.K2_DestroyActor`))

(fn `UserConstructionScript`)